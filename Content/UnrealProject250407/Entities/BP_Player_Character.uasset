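; Player character Blueprint that handles movement, camera look, jumping, sprinting and weapon slot selection through Enhanced Input.
; Look applies yaw to the controller and clamped pitch directly to the camera, with separate sensitivities.
; A timeline ramps max walk speed for sprinting.
; An inventory struct holds weapon classes and a selected index for three hotkeys; adding or selecting only updates this data and prints debug text, without spawning weapons.
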(event `self.ReceiveBeginPlay`
  ; Get Player Controller, Not sure if It's Needed but we Store it Anyway
  (bind _aspc_player_controller (cast `/Game/UnrealProject250407/Entities/PC_Player_Controller` (`GameplayStatics.GetPlayerController` 0)))
  (set `self.PC_Player Controller` _aspc_player_controller))

(event `EnhancedInput|/Game/UnrealProject250407/Input/IA_Move`
  (params (ActionValue :type "Vector2D Structure") (ElapsedSeconds :type "Float (double-precision)") (TriggeredSeconds :type "Float (double-precision)") (InputAction :type "InputAction Object Reference" :default "/Game/UnrealProject250407/Input/IA_Move.IA_Move"))
  (bind (_returnvalue_roll _returnvalue_pitch _returnvalue_yaw) (`KismetMathLibrary.BreakRotator` (`self.GetControlRotation`)))
  ; Handle Player Movement
  (:`Triggered`
    (`self.AddMovementInput` (`KismetMathLibrary.Conv_RotatorToVector` (`self.GetControlRotation`)) ActionValue_Y)
    (`self.AddMovementInput` (`KismetMathLibrary.GetRightVector` (`KismetMathLibrary.MakeRotator` _returnvalue_roll 0.0 _returnvalue_yaw)) ActionValue_X)))

(event `EnhancedInput|/Game/UnrealProject250407/Input/IA_Look`
  (params (ActionValue :type "Vector2D Structure") (ElapsedSeconds :type "Float (double-precision)") (TriggeredSeconds :type "Float (double-precision)") (InputAction :type "InputAction Object Reference" :default "/Game/UnrealProject250407/Input/IA_Look.IA_Look"))
  (bind _camera (`self.Camera`))
  (bind (_relativerotation_roll _relativerotation_pitch) (`KismetMathLibrary.BreakRotator` (`SceneComponent.RelativeRotation` _camera)))
  ; Handle Camera Movement, Separate Camera Sensitivity since Visible Speed is Different for Pitch
  (:`Triggered`
    (`self.AddControllerYawInput` (* ActionValue_X (`self.iCameraSensitivityYaw`)))
    (`SceneComponent.K2_AddRelativeRotation` (`self.Camera`) (`KismetMathLibrary.MakeRotator` 0.0 (* ActionValue_Y (`self.iCameraSensitivityPitch`))) false false)
    ; Clamp Camera to Stop it from Inverting
    (`SceneComponent.K2_SetRelativeRotation` _camera (`KismetMathLibrary.MakeRotator` 0.0 (`KismetMathLibrary.FClamp` _relativerotation_pitch -70.0 70.0)) false false)))

(event `EnhancedInput|/Game/UnrealProject250407/Input/IA_Jump`
  (params (ActionValue :type Boolean) (ElapsedSeconds :type "Float (double-precision)") (TriggeredSeconds :type "Float (double-precision)") (InputAction :type "InputAction Object Reference" :default "/Game/UnrealProject250407/Input/IA_Jump.IA_Jump"))
  ; Handle Jumping
  (:`Started`
    (`self.Jump`))
  (:`Completed`
    (`self.StopJumping`)))

(event `EnhancedInput|/Game/UnrealProject250407/Input/IA_Select_Weapon_1`
  (params (ActionValue :type Boolean) (ElapsedSeconds :type "Float (double-precision)") (TriggeredSeconds :type "Float (double-precision)") (InputAction :type "InputAction Object Reference" :default "/Game/UnrealProject250407/Input/IA_Select_Weapon_1.IA_Select_Weapon_1"))
  (bind (_inventorystruct_iselectedweapon _inventorystruct_aweaponinventory) (break `/Game/UnrealProject250407/Entities/BP_Player_Inventory` (`self.InventoryStruct`)))
  (:`Completed`
    (set `self.InventoryStruct` (make `/Game/UnrealProject250407/Entities/BP_Player_Inventory` 0 _inventorystruct_aweaponinventory))
    (`self.Get_Current_Weapon` :!label _label)))

(event `EnhancedInput|/Game/UnrealProject250407/Input/IA_Select_Weapon_2`
  (params (ActionValue :type Boolean) (ElapsedSeconds :type "Float (double-precision)") (TriggeredSeconds :type "Float (double-precision)") (InputAction :type "InputAction Object Reference" :default "/Game/UnrealProject250407/Input/IA_Select_Weapon_2.IA_Select_Weapon_2"))
  (bind (_inventorystruct_iselectedweapon _inventorystruct_aweaponinventory) (break `/Game/UnrealProject250407/Entities/BP_Player_Inventory` (`self.InventoryStruct`)))
  (:`Completed`
    (set `self.InventoryStruct` (make `/Game/UnrealProject250407/Entities/BP_Player_Inventory` 1 _inventorystruct_aweaponinventory))
    (goto _label)))

(event `EnhancedInput|/Game/UnrealProject250407/Input/IA_Sprint`
  (params (ActionValue :type Boolean) (ElapsedSeconds :type "Float (double-precision)") (TriggeredSeconds :type "Float (double-precision)") (InputAction :type "InputAction Object Reference" :default "/Game/UnrealProject250407/Input/IA_Sprint.IA_Sprint"))
  ; Handle Sprinting
  (:`Started`
    (bind (_direction _walkspeed) (`Timeline|Walk Speed Blend` :!label _label_2) ; Make the Speed Adjustment a Curve
      (:`Update`
        (set `CharacterMovementComponent.MaxWalkSpeed` _walkspeed (`self.CharacterMovement`)))))
  (:`Completed`
    (goto _label_2 :!via `ReverseFromEnd`)))

(event `EnhancedInput|/Game/UnrealProject250407/Input/IA_Select_Weapon_3`
  (params (ActionValue :type Boolean) (ElapsedSeconds :type "Float (double-precision)") (TriggeredSeconds :type "Float (double-precision)") (InputAction :type "InputAction Object Reference" :default "/Game/UnrealProject250407/Input/IA_Select_Weapon_3.IA_Select_Weapon_3"))
  (bind (_inventorystruct_iselectedweapon _inventorystruct_aweaponinventory) (break `/Game/UnrealProject250407/Entities/BP_Player_Inventory` (`self.InventoryStruct`)))
  (:`Completed`
    (set `self.InventoryStruct` (make `/Game/UnrealProject250407/Entities/BP_Player_Inventory` 2 _inventorystruct_aweaponinventory))
    (goto _label)))

(fn `Add_Weapon_To_Inventory`
  (params (WeaponBlueprint :type "/Game/UnrealProject250407/Weapons/BP_Weapon_Base Class Reference"))
  (bind (_inventorystruct_iselectedweapon _inventorystruct_aweaponinventory) (break `/Game/UnrealProject250407/Entities/BP_Player_Inventory` (`self.InventoryStruct`)))
  (bind (_iselectedweapon _aweaponinventory) (break `/Game/UnrealProject250407/Entities/BP_Player_Inventory` (`self.InventoryStruct`)))
  (bind _returnvalue (`KismetArrayLibrary.Array_Add` _aweaponinventory WeaponBlueprint))
  (set `self.InventoryStruct` (make `/Game/UnrealProject250407/Entities/BP_Player_Inventory` _iselectedweapon _inventorystruct_aweaponinventory))
  ; Debug
  (`KismetSystemLibrary.PrintString` (`KismetStringLibrary.Concat_StrStr` "Slot " (`KismetStringLibrary.Conv_IntToString` _returnvalue) ": " (`KismetSystemLibrary.GetClassDisplayName` WeaponBlueprint))))

(fn `Get_Current_Weapon`
  (returns (CurrentWeaponBlueprint :type "/Game/UnrealProject250407/Weapons/BP_Weapon_Base Class Reference"))
  (bind (_inventorystruct_iselectedweapon _inventorystruct_aweaponinventory) (break `/Game/UnrealProject250407/Entities/BP_Player_Inventory` (`self.InventoryStruct`)))
  (bind _output (`|GetArrayItem` _inventorystruct_aweaponinventory _inventorystruct_iselectedweapon))
  (`KismetSystemLibrary.PrintString` (`KismetStringLibrary.Concat_StrStr` "Selected Slot  " (`KismetStringLibrary.Conv_IntToString` _inventorystruct_iselectedweapon) ": " (`KismetSystemLibrary.GetClassDisplayName` _output)))
  (return _output))

(fn `UserConstructionScript`)